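; Menu game mode that starts data preloading on the cube data singleton and platform login through the game instance on BeginPlay.
; ForceLevelUIReload refreshes level selection through the menu HUD, using either the new main menu with the saved classic player mode or the older standard and advanced widgets.
; It registers only the randomised floor-piece family, using one transition piece for start and end, and leaves floor-piece class registration empty.
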(event `self.ReceiveBeginPlay`
  (bind _ascube_data_singleton_bp (cast `/Game/Blueprints/Core/CubeDataSingletonBP` (`CubeSingletonDataLibrary.GetSingletonGameData`))
    (:`then`
      (`/Game/Blueprints/Core/CubeDataSingletonBP.PreloadTest` _ascube_data_singleton_bp)
      (bind _ascube_game_instance_bp (cast `/Game/Blueprints/Core/CubeGameInstanceBP` (`GameplayStatics.GetGameInstance`)))
      (`/Game/Blueprints/Core/CubeGameInstanceBP.LoginPlatform` _ascube_game_instance_bp)
      (`CubeSingletonDataLibrary.CustomLog` "Menu GM Beginplay" "Warn"))
    (:`CastFailed`
      (`CubeSingletonDataLibrary.CustomLog` "Cube Dat Singleton class invalid" "Error"))))

(event `self.ForceLevelUIReload`
  (bind _asmenu_hudbp (cast `/Game/Blueprints/Menu/MenuHUDBP` (`PlayerController.GetHUD` (`GameplayStatics.GetPlayerController` 0)))
    (:`then`
      (`CubeSingletonDataLibrary.CustomLog` "UI Reloaded")
      (if (`/Game/Blueprints/Menu/MenuHUDBP.NewHud` _asmenu_hudbp)
        (bind _ascube_game_instance_bp (cast `/Game/Blueprints/Core/CubeGameInstanceBP` (`GameplayStatics.GetGameInstance`)))
        (bind _newmainmenuwidget (`/Game/Blueprints/Menu/MenuHUDBP.NewMainMenuWidget` _asmenu_hudbp))
        (bind _classicplayermode (`CubeGameInstance.ClassicPlayerMode` _ascube_game_instance_bp))
        (`/Game/Blueprints/Menu/NewMainMenuWidgetBP.SetPlayerMode` _newmainmenuwidget _classicplayermode)
        (`/Game/Blueprints/Menu/NewMainMenuWidgetBP.LoadLevels` _newmainmenuwidget _classicplayermode)
        (else
          (bind _levelselectwidget (`/Game/Blueprints/Menu/MenuHUDBP.LevelSelectWidget` _asmenu_hudbp))
          (`/Game/Blueprints/Menu/LevelSelectWidgetBP.SetPlayerMode` _levelselectwidget false)
          (`/Game/Blueprints/Menu/LevelSelectWidgetBP.LoadLevels` _levelselectwidget true)
          (bind _levelselectwidgetadvanced (`/Game/Blueprints/Menu/MenuHUDBP.LevelSelectWidgetAdvanced` _asmenu_hudbp))
          (`/Game/Blueprints/Menu/LevelSelectWidgetBP.SetPlayerMode` _levelselectwidgetadvanced false)
          (`/Game/Blueprints/Menu/LevelSelectWidgetBP.LoadLevels` _levelselectwidgetadvanced false))))
    (:`CastFailed`
      (`CubeSingletonDataLibrary.CustomLog` "UI RELOAD: CAST FAILED" "Error"))))

(event `self.RegisterFloorPieceFamilies`
  (`self.RegisterFamily` "/Game/Blueprints/Objects/FloorPieces/Special/RandomisedTransitionFloorPieceBP.RandomisedTransitionFloorPieceBP_C" "/Game/Blueprints/Objects/FloorPieces/Special/RandomisedTransitionFloorPieceBP.RandomisedTransitionFloorPieceBP_C" "EPF_RANDOMISED"))

(event `self.RegisterFloorPieceClasses`)

(fn `UserConstructionScript`)