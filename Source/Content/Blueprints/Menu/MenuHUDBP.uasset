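; Menu HUD that creates and switches the game's menu widgets and opens platform leaderboards, prompting login when needed.
; BeginPlay shows a loading widget and builds either the new or legacy widget set per NewHud; LoadingFinished swaps in the main menu and loads levels.
; The legacy path jumps to Classic or Advanced level select when returning from gameplay, using GameInstance flags.
; Despite its name, FadeBetweenWidgets switches instantly, ignoring its Instant parameter.
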(event `LoadingFinished`
  (bind _levelselectwidget (`self.LevelSelectWidget`))
  (bind _newmainmenuwidget (`self.NewMainMenuWidget`))
  (bind _mainmenuwidget (`self.MainMenuWidget`))
  (`CubeSingletonDataLibrary.CustomLog` "LoadingFinished")
  (if (`self.NewHud`)
    (`UserWidget.AddToViewport` _newmainmenuwidget 0)
    (set `self.CurrentWidget` _newmainmenuwidget)
    (`Widget.RemoveFromParent` (`self.LoadingWidget`))
    (bind _ascube_game_instance_bp (cast `/Game/Blueprints/Core/CubeGameInstanceBP` (`GameplayStatics.GetGameInstance`)))
    (set `CubeGameInstance.MenuLoadedFromGame` false _ascube_game_instance_bp)
    (bind _classicplayermode (`CubeGameInstance.ClassicPlayerMode` _ascube_game_instance_bp))
    (`/Game/Blueprints/Menu/NewMainMenuWidgetBP.LoadLevels` _newmainmenuwidget _classicplayermode)
    (`/Game/Blueprints/Menu/NewMainMenuWidgetBP.SetPlayerMode` _newmainmenuwidget _classicplayermode)
    (`/Game/Blueprints/Menu/NewMainMenuWidgetBP.SelectLevel` _newmainmenuwidget -1 -1)
    (else
      (`UserWidget.AddToViewport` _mainmenuwidget 0)
      (set `self.CurrentWidget` _mainmenuwidget)
      (`Widget.RemoveFromParent` (`self.LoadingWidget`))
      (`/Game/Blueprints/Menu/LevelSelectWidgetBP.LoadLevels` (`self.LevelSelectWidget`) true)
      (`/Game/Blueprints/Menu/LevelSelectWidgetBP.LoadLevels` (`self.LevelSelectWidgetAdvanced`) false)
      (bind _ascube_game_instance_bp_2 (cast `/Game/Blueprints/Core/CubeGameInstanceBP` (`GameplayStatics.GetGameInstance`)))
      (if (`CubeGameInstance.MenuLoadedFromGame` _ascube_game_instance_bp_2)
        (set `CubeGameInstance.MenuLoadedFromGame` false _ascube_game_instance_bp_2)
        (bind _classicplayermode_2 (`CubeGameInstance.ClassicPlayerMode` _ascube_game_instance_bp_2))
        (`self.FadeBetweenWidgets` (`self.MainMenuWidget`) (select `bool` _classicplayermode_2 :`false` (`self.LevelSelectWidgetAdvanced`) :`true` _levelselectwidget) true)
        (`/Game/Blueprints/Menu/LevelSelectWidgetBP.SetPlayerMode` _levelselectwidget _classicplayermode_2)
        (`/Game/Blueprints/Menu/LevelSelectWidgetBP.SetPlayerMode` (select `bool` _classicplayermode_2 :`false` (`self.LevelSelectWidgetAdvanced`) :`true` _levelselectwidget) _classicplayermode_2)
        (`/Game/Blueprints/Menu/LevelSelectWidgetBP.SelectLevel` _levelselectwidget 0 null)
        (`/Game/Blueprints/Menu/LevelSelectWidgetBP.SelectLevel` (select `bool` _classicplayermode_2 :`false` (`self.LevelSelectWidgetAdvanced`) :`true` _levelselectwidget) 0 null)))))

(event `self.ReceiveBeginPlay`
  (bind _returnvalue (`GameplayStatics.GetPlayerController` 0))
  (bind _returnvalue_2 (`GameplayStatics.GetPlayerController` 0))
  (bind _returnvalue_3 (`GameplayStatics.GetPlayerController` 0))
  (bind _returnvalue_4 (`|CreateWidget` "/Game/Blueprints/Menu/LoadingLevelWidgetBP.LoadingLevelWidgetBP_C" _returnvalue_3))
  (bind _output_get (set `self.LoadingWidget` _returnvalue_4))
  (`UserWidget.AddToViewport` _output_get 0)
  (if (`self.NewHud`)
    (bind _returnvalue_5 (`|CreateWidget` "/Game/Blueprints/Menu/NewMainMenuWidgetBP.NewMainMenuWidgetBP_C" _returnvalue_3))
    (set `self.NewMainMenuWidget` _returnvalue_5)
    (`|ExecutionSequence` :!label _label
      (:`then_0`
        (bind _returnvalue_6 (`|CreateWidget` "/Game/Blueprints/Menu/OptionsWidgetBP.OptionsWidgetBP_C" _returnvalue_2))
        (set `self.OptionsWidget` _returnvalue_6))
      (:`then_1`
        (bind _returnvalue_7 (`|CreateWidget` "/Game/Blueprints/Menu/StatisticsWidgetBP.StatisticsWidgetBP_C" _returnvalue_2))
        (set `self.AchievementsWidget` _returnvalue_7)))
    (else
      (`|ExecutionSequence`
        (:`then_0`
          (goto _label))
        (:`then_1`
          (bind _returnvalue_8 (`|CreateWidget` "/Game/Blueprints/Menu/PlayWidgetBP.PlayWidgetBP_C" _returnvalue))
          (set `self.PlayWidget` _returnvalue_8))
        (:`then_2`
          (bind _returnvalue_9 (`|CreateWidget` "/Game/Blueprints/Menu/LevelSelectWidgetBP.LevelSelectWidgetBP_C" _returnvalue))
          (set `self.LevelSelectWidget` _returnvalue_9))
        (:`then_3`
          (bind _returnvalue_10 (`|CreateWidget` "/Game/Blueprints/Menu/LevelSelectWidgetBP.LevelSelectWidgetBP_C" _returnvalue))
          (set `self.LevelSelectWidgetAdvanced` _returnvalue_10))
        (:`then_4`
          (bind _returnvalue_11 (`|CreateWidget` "/Game/Blueprints/Menu/MenuWidgetBP.MenuWidgetBP_C" _returnvalue))
          (set `self.MainMenuWidget` _returnvalue_11))))))

(event `self.ReceiveTick`
  (params (DeltaSeconds :type "Float (single-precision)")))

(event `LoadHighscores`
  (params (Classic :type Boolean))
  (bind _returnvalue (`GameplayStatics.GetPlayerController` 0))
  (if (`KismetSystemLibrary.IsLoggedIn` _returnvalue)
    (if Classic :!label _label_2
      (`KismetSystemLibrary.ShowPlatformSpecificLeaderboardScreen` "ClassicMode")
      (else
        (`KismetSystemLibrary.ShowPlatformSpecificLeaderboardScreen` "AdvancedMode")))
    (else
      (`ShowLoginUICallbackProxy.ShowExternalLoginUI` _returnvalue
        (:`OnSuccess`
          (`CubeSingletonDataLibrary.CustomLog` "Successfully logged in!")
          (goto _label_2))
        (:`OnFailure`
          (`CubeSingletonDataLibrary.CustomLog` "Failed to log in!" "Warn"))))))

(fn `FadeBetweenWidgets`
  (params (WidgetFrom :type "/Game/Blueprints/UI/CubeUserWidget Object Reference") (WidgetTo :type "/Game/Blueprints/UI/CubeUserWidget Object Reference") (Instant :type Boolean))
  (if (not (`self.NewHud`))
    (`Widget.RemoveFromParent` WidgetFrom)
    (`Widget.SetVisibility` WidgetFrom "Hidden"))
  (`Widget.SetVisibility` WidgetTo "Visible")
  (`UserWidget.AddToViewport` WidgetTo 0)
  (bind _output_get (set `self.CurrentWidget` WidgetTo))
  (`/Game/Blueprints/UI/CubeUserWidget.OnReload` WidgetTo)
  (`/Game/Blueprints/UI/CubeUserWidget.OnReload` _output_get))

(fn `ReturnToMainMenu`
  (params (From :type "/Game/Blueprints/UI/CubeUserWidget Object Reference"))
  (bind _newhud (`self.NewHud`))
  (bind _returnvalue (select `bool` _newhud :`false` (`self.MainMenuWidget`) :`true` (`self.NewMainMenuWidget`) :!type "/Game/Blueprints/UI/CubeUserWidget Object Reference"))
  (`Widget.RemoveFromParent` From)
  (if (not _newhud)
    (`Widget.SetVisibility` _returnvalue "Visible")
    (`UserWidget.AddToViewport` _returnvalue 0))
  (set `self.CurrentWidget` _returnvalue)
  (`/Game/Blueprints/UI/CubeUserWidget.OnReload` _returnvalue))

(fn `UserConstructionScript`)