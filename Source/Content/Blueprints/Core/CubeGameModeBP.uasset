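; Game mode for an endless and level-based cube runner with Classic and Advanced modes.
; Registers floor piece families and weighted, difficulty-rated classes, and builds hand-authored levels by queuing pieces, including split paths, with speed options.
; On game end it drives HUD titles, game-over screen and ad banner, updating highscores, leaderboards and achievements after crashes.
; It also applies per-level fog opacity shortly after BeginPlay and shows upgrade pickup titles.
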(event `SetFogOpacity`
  (bind _fog (`self.GetFogActor`))
  (`/Engine/EditorBlueprintResources/StandardMacros.IsValid` _fog
    (:`Is Valid`
      (`ExponentialHeightFogComponent.SetFogMaxOpacity` (`ExponentialHeightFog.Component` _fog) (`self.LevelFogOpacity`)))))

(event `self.ReceiveBeginPlay`
  (`|ExecutionSequence`
    (:`then_0`
      (`KismetSystemLibrary.K2_SetTimerDelegate` (delegate `SetFogOpacity`) 0.01))
    (:`then_1`
      (bind _ascube_data_singleton_bp (cast `/Game/Blueprints/Core/CubeDataSingletonBP` (`CubeSingletonDataLibrary.GetSingletonGameData`)))
      (`/Game/Blueprints/Core/CubeDataSingletonBP.PreloadTest` _ascube_data_singleton_bp)
      (bind _ascube_gameplay_hudbp (cast `/Game/Blueprints/UI/CubeGameplayHUDBP` (`PlayerController.GetHUD` (`GameplayStatics.GetPlayerController` 0))))
      (bind _loadingwidget (`/Game/Blueprints/UI/CubeGameplayHUDBP.LoadingWidget` _ascube_gameplay_hudbp))
      (`/Engine/EditorBlueprintResources/StandardMacros.IsValid` _loadingwidget
        (:`Is Valid`
          (`Widget.RemoveFromParent` _loadingwidget))
        (:`Is Not Valid`
          _))
      (`KismetSystemLibrary.K2_SetTimer` _ascube_gameplay_hudbp "HideTitle" 5.0)
      (if (`CubeSingletonDataLibrary.IsWithEditor`)
        _))))

(event `self.GameEnd`
  (params (Reason :type "EGameEndState Enum" :default "EGES_FAIL"))
  (bind _returnvalue (`GameplayStatics.GetPlayerController` 0))
  (bind _playerref (`self.PlayerRef`))
  (bind _returnvalue_2 (`KismetMathLibrary.FFloor` (/ (`BasePlayerPawn.TotalDistanceTravelled` _playerref) 100.0)))
  (if (`BasePlayerPawn.IsAlive` _playerref)
    (`parent.GameEnd` Reason)
    (set `PlayerController.bShowMouseCursor` true _returnvalue)
    (`KismetSystemLibrary.ShowAdBanner` 0 true)
    (bind _ascube_gameplay_hudbp (cast `/Game/Blueprints/UI/CubeGameplayHUDBP` (`PlayerController.GetHUD` _returnvalue)))
    (bind _ascube_game_instance_bp (cast `/Game/Blueprints/Core/CubeGameInstanceBP` (`GameplayStatics.GetGameInstance`)))
    (switch `EGameEndState` Reason
      (:`EGES_FAIL`
        (bind _mainhudwidget (`/Game/Blueprints/UI/CubeGameplayHUDBP.MainHUDWidget` _ascube_gameplay_hudbp))
        (`/Game/Blueprints/UI/CubeGameplayHUDBP.QueueTitle` _ascube_gameplay_hudbp (`KismetTextLibrary.Conv_TextToString` (`/Game/Blueprints/UI/CubeGameplayHUDWidgetBP.GetText_0` _mainhudwidget)) -1.0)
        (bind _returnvalue_3 (== (`CubeGameInstance.LevelIndex` _ascube_game_instance_bp) -1))
        (`/Game/Blueprints/UI/CubeGameplayHUDBP.ShowGameOver` _ascube_gameplay_hudbp false _returnvalue_3)
        (bind _classicplayermode (`CubeGameInstance.ClassicPlayerMode` _ascube_game_instance_bp))
        (if _classicplayermode
          (if (> _returnvalue_2 (`CubeGameInstance.ClassicHighscore` _ascube_game_instance_bp))
            (set `CubeGameInstance.AdvancedHighscore` _returnvalue_2 _ascube_game_instance_bp)
            (if (`KismetSystemLibrary.IsLoggedIn` (`GameplayStatics.GetPlayerController` 0)) :!label _label
              (`LeaderboardBlueprintLibrary.WriteLeaderboardInteger` (`GameplayStatics.GetPlayerController` 0) (select `bool` _classicplayermode :`false` "AdvancedMode" :`true` "ClassicMode") _returnvalue_2))
            (`/Game/Blueprints/Core/CubeGameInstanceBP.UpdateAchievements` _ascube_game_instance_bp)
            (if _returnvalue_3
              (`Widget.SetVisibility` (`/Game/Blueprints/UI/CubeGameplayHUDWidgetBP.NewRecord_Text` _mainhudwidget) "Visible")))
          (elif (> _returnvalue_2 (`CubeGameInstance.AdvancedHighscore` _ascube_game_instance_bp))
            (set `CubeGameInstance.ClassicHighscore` _returnvalue_2 _ascube_game_instance_bp)
            (goto _label))))
      (:`EGES_SUCCESS`
        (`/Game/Blueprints/UI/CubeGameplayHUDBP.QueueTitle` _ascube_gameplay_hudbp "Level Complete" -1.0)
        (`/Game/Blueprints/UI/CubeGameplayHUDBP.ShowGameOver` _ascube_gameplay_hudbp true _returnvalue_3)
        (`Widget.SetVisibility` (`/Game/Blueprints/UI/CubeGameplayHUDWidgetBP.NewRecord_Text` _mainhudwidget) "Hidden")))))

(event `self.OnUpgradeAdded`
  (params (Upgrade :type "BaseUpgrade Object Reference"))
  (bind _ascube_gameplay_hudbp (cast `/Game/Blueprints/UI/CubeGameplayHUDBP` (`PlayerController.GetHUD` (`GameplayStatics.GetPlayerController` 0))))
  (bind _returnvalue (`BaseUpgrade.GetUpgradeDisplayName` Upgrade))
  (`/Game/Blueprints/UI/CubeGameplayHUDBP.QueueTitle` _ascube_gameplay_hudbp _returnvalue 2.5))

(event `self.RegisterFloorPieceFamilies`
  (`self.RegisterFamiliesBP`))

(event `self.RegisterFloorPieceClasses`
  (`self.RegisterClassesBP`))

(event `self.LoadClassicLevel`
  (params (Level :type Integer))
  (`self.LoadClassicLevelBP` Level))

(event `self.LoadAdvancedLevel`
  (params (Level :type Integer))
  (`self.LoadAdvancedLevelBP` Level))

(event `IncrementAddictedAchievement`
  (bind _returnvalue (`GameplayStatics.GetPlayerController` 0))
  (if (`KismetSystemLibrary.IsLoggedIn` _returnvalue)
    (`AchievementWriteCallbackProxy.WriteAchievementProgress` _returnvalue "Addicted" 1.0
      (:`OnSuccess`
        (`CubeSingletonDataLibrary.CustomLog` "Succesful write \"Addicted\" achievement")
        (if true
          (if true
            _)))
      (:`OnFailure`
        (`CubeSingletonDataLibrary.CustomLog` "Failed to write \"Addicted\" achievement")))))

(fn `GetFogActor`
  (returns (Fog :type "ExponentialHeightFog Object Reference"))
  (`/Engine/EditorBlueprintResources/StandardMacros.IsValid` (`self.FogActor`)
    (:`Is Valid`
      _)
    (:`Is Not Valid`
      (bind _outactors (`GameplayStatics.GetAllActorsOfClass` "/Script/Engine.ExponentialHeightFog"))
      (set `self.FogActor` (`|GetArrayItem` _outactors))))
  (return (`self.FogActor`)))

(fn `LoadAdvancedLevelBP`
  (params (Level :type Integer))
  (switch `int` Level
    (:`Default`
      (`CubeSingletonDataLibrary.CustomLog` (`KismetStringLibrary.BuildString_Int` "" "Unhandled level selected! Level Index: ") "Error"))
    (:`0`
      (`self.SetLevelOptions` true 1500.0 30.0 true)
      (`self.QueuePieceSplitWithVariation` "/Game/Blueprints/Objects/FloorPieces/Cube/StraightFloorPieceBP.StraightFloorPieceBP_C" 1)
      (`self.QueuePieceSplitWithVariation` "/Game/Blueprints/Objects/FloorPieces/Cube/LeftTurnFloorPieceBP2.LeftTurnFloorPieceBP2_C")
      (`self.QueuePieceSplitWithVariation` "/Game/Blueprints/Objects/FloorPieces/Cube/StraightFloorPieceBP.StraightFloorPieceBP_C" 5)
      (`self.QueuePiece` "/Game/Blueprints/Objects/FloorPieces/Special/RandomisedFloorPieceBP.RandomisedFloorPieceBP_C")
      (`self.QueuePieceSplitWithVariation` "/Game/Blueprints/Objects/FloorPieces/Cube/RightTurnFloorPieceBP.RightTurnFloorPieceBP_C" 1)
      (`self.QueuePieceSplitWithVariation` "/Game/Blueprints/Objects/FloorPieces/Cube/StraightFloorPieceBP.StraightFloorPieceBP_C" 5)
      (`self.QueuePiece` "/Game/Blueprints/Objects/FloorPieces/Special/LevelEndFloorPieceBP.LevelEndFloorPieceBP_C"))
    (:`7`
      (`self.SetLevelOptions` true 3100.0 10.0 false (0.0 0.0 0.0) (struct) false)
      (`self.QueuePiece` "/Game/Blueprints/Objects/FloorPieces/Platform/StraightPlatformFloorPieceBP.StraightPlatformFloorPieceBP_C")
      (`self.QueuePieceSplitWithVariation` "/Game/Blueprints/Objects/FloorPieces/Platform/DiagonalPlatformFloorPieceBP.DiagonalPlatformFloorPieceBP_C" 1)
      (`self.QueuePieceSplitWithVariation` "/Game/Blueprints/Objects/FloorPieces/Platform/StraightPlatformFloorPieceBP.StraightPlatformFloorPieceBP_C" 1)
      (`self.QueuePiece` "/Game/Blueprints/Objects/FloorPieces/Platform/JumpPlatformFloorPieceBP1.JumpPlatformFloorPieceBP1_C")
      (`self.QueuePieceSplitWithVariation` "/Game/Blueprints/Objects/FloorPieces/Platform/StraightPlatformFloorPieceBP.StraightPlatformFloorPieceBP_C" 2)
      (`self.QueuePieceSplitWithVariation` "/Game/Blueprints/Objects/FloorPieces/Platform/StraightPlatformFloorPieceBP.StraightPlatformFloorPieceBP_C" 3)
      (`self.QueuePieceSplitWithVariation` "/Game/Blueprints/Objects/FloorPieces/Platform/PlatformLeftTurnFloorPieceBP.PlatformLeftTurnFloorPieceBP_C")
      (`self.QueuePieceSplitWithVariation` "/Game/Blueprints/Objects/FloorPieces/Platform/PlatformLeftTurnFloorPieceBP.PlatformLeftTurnFloorPieceBP_C")
      (`self.QueuePiece` "/Game/Blueprints/Objects/FloorPieces/Platform/JumpPlatformFloorPieceBP1.JumpPlatformFloorPieceBP1_C")
      (`self.QueuePieceSplitWithVariation` "/Game/Blueprints/Objects/FloorPieces/Platform/StraightPlatformFloorPieceBP.StraightPlatformFloorPieceBP_C" 4)
      (`self.QueuePieceSplitWithVariation` "/Game/Blueprints/Objects/FloorPieces/Platform/StraightPlatformFloorPieceBP.StraightPlatformFloorPieceBP_C" 5)
      (`self.QueuePiece` "/Game/Blueprints/Objects/FloorPieces/Platform/PlatformLevelEndFloorPieceBP.PlatformLevelEndFloorPieceBP_C"))))

(fn `LoadClassicLevelBP`
  (params (Level :type Integer))
  (switch `int` Level
    (:`Default`
      (`CubeSingletonDataLibrary.CustomLog` (`KismetStringLibrary.BuildString_Int` "" "Unhandled level selected! Level Index: " Level) "Error"))
    (:`0`
      ;[1 1 1] Green
      (`self.QueuePieceMulti` "/Game/Blueprints/Objects/FloorPieces/Special/RandomisedFloorPieceBP.RandomisedFloorPieceBP_C" 2)
      (`self.QueuePiece` "/Game/Blueprints/Objects/FloorPieces/Special/LevelEndFloorPieceBP.LevelEndFloorPieceBP_C")
      (`self.SetLevelOptions` false 900.0 20.0 true))
    (:`1`
      (`self.QueuePiece` "/Game/Blueprints/Objects/FloorPieces/Special/RandomisedFloorPieceBP.RandomisedFloorPieceBP_C")
      (`self.QueuePieceWithVariation` "/Game/Blueprints/Objects/FloorPieces/Cube/StraightFloorPieceBP.StraightFloorPieceBP_C" 5)
      (`self.QueuePiece` "/Game/Blueprints/Objects/FloorPieces/Cube/LeftTurnFloorPieceBP.LeftTurnFloorPieceBP_C")
      (`self.QueuePiece` "/Game/Blueprints/Objects/FloorPieces/Special/RandomisedFloorPieceBP.RandomisedFloorPieceBP_C")
      (`self.QueuePiece` "/Game/Blueprints/Objects/FloorPieces/Special/LevelEndFloorPieceBP.LevelEndFloorPieceBP_C")
      (`self.SetLevelOptions` true 1000.0 20.0 true))
    (:`2`
      (`self.QueuePiece` "/Game/Blueprints/Objects/FloorPieces/Special/RandomisedFloorPieceBP.RandomisedFloorPieceBP_C")
      (`self.QueuePiece` "/Game/Blueprints/Objects/FloorPieces/Cube/SBendFloorPieceBP.SBendFloorPieceBP_C")
      (`self.QueuePiece` "/Game/Blueprints/Objects/FloorPieces/Special/RandomisedFloorPieceBP.RandomisedFloorPieceBP_C")
      (`self.QueuePieceWithVariation` "/Game/Blueprints/Objects/FloorPieces/Cube/RightTurnFloorPieceBP.RightTurnFloorPieceBP_C" 1)
      (`self.QueuePieceWithVariation` "/Game/Blueprints/Objects/FloorPieces/Cube/LeftTurnFloorPieceBP.LeftTurnFloorPieceBP_C" 1)
      (`self.QueuePiece` "/Game/Blueprints/Objects/FloorPieces/Special/RandomisedFloorPieceBP.RandomisedFloorPieceBP_C")
      (`self.QueuePiece` "/Game/Blueprints/Objects/FloorPieces/Special/LevelEndFloorPieceBP.LevelEndFloorPieceBP_C")
      (`self.SetLevelOptions` true 1000.0 30.0 true))
    (:`3`
      (`self.QueuePiece` "/Game/Blueprints/Objects/FloorPieces/Cube/CubeTransitionFloorPieceBP.CubeTransitionFloorPieceBP_C")
      (`self.QueuePieceMulti` "/Game/Blueprints/Objects/FloorPieces/Cube/LeftTurnFloorPieceBP2.LeftTurnFloorPieceBP2_C" 6)
      (`self.QueuePiece` "/Game/Blueprints/Objects/FloorPieces/Cube/CubeEndTransitionFloorPieceBP.CubeEndTransitionFloorPieceBP_C")
      (`self.QueuePieceMulti` "/Game/Blueprints/Objects/FloorPieces/Special/RandomisedFloorPieceBP.RandomisedFloorPieceBP_C" 2)
      (`self.QueuePiece` "/Game/Blueprints/Objects/FloorPieces/Special/LevelEndFloorPieceBP.LevelEndFloorPieceBP_C")
      (`self.SetLevelOptionsWithPreSpawn` 1 700.0 100.0))
    (:`4`
      ;[1 1 1] Blue
      (`self.QueuePiece` "/Game/Blueprints/Objects/FloorPieces/Special/RandomisedFloorPieceBP.RandomisedFloorPieceBP_C")
      (`self.QueuePieceWithVariation` "/Game/Blueprints/Objects/FloorPieces/Cube/SBendFloorPieceBP.SBendFloorPieceBP_C" 1)
      (`self.QueuePieceWithVariation` "/Game/Blueprints/Objects/FloorPieces/Cube/LeftTurnFloorPieceBP.LeftTurnFloorPieceBP_C" 1)
      (`self.QueuePieceWithVariation` "/Game/Blueprints/Objects/FloorPieces/Cube/RightTurnFloorPieceBP.RightTurnFloorPieceBP_C" 1)
      (`self.QueuePieceWithVariation` "/Game/Blueprints/Objects/FloorPieces/Cube/StraightFloorPieceBP.StraightFloorPieceBP_C" 1)
      (`self.QueuePiece` "/Game/Blueprints/Objects/FloorPieces/Special/RandomisedFloorPieceBP.RandomisedFloorPieceBP_C")
      (`self.QueuePiece` "/Game/Blueprints/Objects/FloorPieces/Special/LevelEndFloorPieceBP.LevelEndFloorPieceBP_C")
      (`self.SetLevelOptions` true 1000.0 30.0 true))
    (:`5`
      (`self.QueuePieceWithVariation` "/Game/Blueprints/Objects/FloorPieces/Cube/StraightFloorPieceBP.StraightFloorPieceBP_C" 1)
      (`self.QueuePiece` "/Game/Blueprints/Objects/FloorPieces/Special/RandomisedFloorPieceBP.RandomisedFloorPieceBP_C")
      (`self.QueuePiece` "/Game/Blueprints/Objects/FloorPieces/Cube/DoubleSBendFloorPieceBP.DoubleSBendFloorPieceBP_C")
      (`self.QueuePiece` "/Game/Blueprints/Objects/FloorPieces/Special/RandomisedFloorPieceBP.RandomisedFloorPieceBP_C")
      (`self.QueuePieceWithVariation` "/Game/Blueprints/Objects/FloorPieces/Cube/StraightFloorPieceBP.StraightFloorPieceBP_C" 1)
      (`self.QueuePiece` "/Game/Blueprints/Objects/FloorPieces/Special/LevelEndFloorPieceBP.LevelEndFloorPieceBP_C")
      (`self.SetLevelOptions` true 1200.0 32.0 true))
    (:`6`
      (`self.QueuePiece` "/Game/Blueprints/Objects/FloorPieces/Special/RandomisedFloorPieceBP.RandomisedFloorPieceBP_C")
      (`self.QueuePiece` "/Game/Blueprints/Objects/FloorPieces/Indoor/ArchesFloorPieceBP.ArchesFloorPieceBP_C")
      (`self.QueuePiece` "/Game/Blueprints/Objects/FloorPieces/Indoor/IndoorFloorPieceBP.IndoorFloorPieceBP_C")
      (`self.QueuePiece` "/Game/Blueprints/Objects/FloorPieces/Special/RandomisedFloorPieceBP.RandomisedFloorPieceBP_C")
      (`self.QueuePiece` "/Game/Blueprints/Objects/FloorPieces/Special/LevelEndFloorPieceBP.LevelEndFloorPieceBP_C")
      (`self.SetLevelOptions` true 1500.0 30.0 true))
    (:`7`
      (`self.QueuePieceMultiWithVariation` "/Game/Blueprints/Objects/FloorPieces/Cube/StraightFloorPieceBP.StraightFloorPieceBP_C" 4 2)
      (`self.QueuePiece` "/Game/Blueprints/Objects/FloorPieces/Indoor/IndoorFloorPieceBP.IndoorFloorPieceBP_C")
      (`self.QueuePiece` "/Game/Blueprints/Objects/FloorPieces/Indoor/IndoorFloorPieceBP2.IndoorFloorPieceBP2_C")
      (`self.QueuePiece` "/Game/Blueprints/Objects/FloorPieces/Special/LevelEndFloorPieceBP.LevelEndFloorPieceBP_C")
      (`self.SetLevelOptions` true 1500.0 50.0 true))
    (:`8`
      ;[1 1 1] Red
      (`self.QueuePieceSplit` "/Game/Blueprints/Objects/FloorPieces/Cube/StraightSplitFloorPieceBP.StraightSplitFloorPieceBP_C")
      (`self.QueuePiece` "/Game/Blueprints/Objects/FloorPieces/Cube/LeftTurnFloorPieceBP.LeftTurnFloorPieceBP_C")
      (`self.QueuePieceWithVariation` "/Game/Blueprints/Objects/FloorPieces/Cube/StraightFloorPieceBP.StraightFloorPieceBP_C" 4)
      (`self.QueuePiece` "/Game/Blueprints/Objects/FloorPieces/Special/LevelEndFloorPieceBP.LevelEndFloorPieceBP_C")
      (`self.EndSplitPieceQueue`)
      (`self.QueuePiece` "/Game/Blueprints/Objects/FloorPieces/Cube/StraightFloorPieceBP.StraightFloorPieceBP_C")
      (`self.QueuePieceWithVariation` "/Game/Blueprints/Objects/FloorPieces/Cube/StraightFloorPieceBP.StraightFloorPieceBP_C" 4)
      (`self.QueuePiece` "/Game/Blueprints/Objects/FloorPieces/Special/LevelEndFloorPieceBP.LevelEndFloorPieceBP_C")
      (`self.SetLevelOptions` false 1500.0 50.0 true))
    (:`9`
      (`self.SetLevelOptions` true 2000.0 50.0 true)
      (`self.QueuePiece` "/Game/Blueprints/Objects/FloorPieces/Indoor/IndoorFloorPieceBP.IndoorFloorPieceBP_C")
      (`self.QueuePiece` "/Game/Blueprints/Objects/FloorPieces/Indoor/TunnelsFloorPieceBP.TunnelsFloorPieceBP_C")
      (`self.QueuePiece` "/Game/Blueprints/Objects/FloorPieces/Indoor/IndoorFloorPieceBP3.IndoorFloorPieceBP3_C")
      (`self.QueuePiece` "/Game/Blueprints/Objects/FloorPieces/Special/RandomisedFloorPieceBP.RandomisedFloorPieceBP_C")
      (`self.QueuePiece` "/Game/Blueprints/Objects/FloorPieces/Special/LevelEndFloorPieceBP.LevelEndFloorPieceBP_C"))
    (:`10`
      (`self.SetLevelOptions` true 2200.0 50.0 true)
      (for _index (range 10)
        (`self.QueuePieceWithVariation` "/Game/Blueprints/Objects/FloorPieces/Special/RandomisedFloorPieceBP.RandomisedFloorPieceBP_C" _index))
      (`self.QueuePiece` "/Game/Blueprints/Objects/FloorPieces/Special/LevelEndFloorPieceBP.LevelEndFloorPieceBP_C"))
    (:`11`
      (`self.SetLevelOptions` true 1700.0 50.0 false (0.0 0.0 500.0) (struct) false)
      (`self.QueuePiece` "/Game/Blueprints/Objects/FloorPieces/Cube/StraightFloorPieceBP.StraightFloorPieceBP_C")
      (`self.QueuePieceWithVariation` "/Game/Blueprints/Objects/FloorPieces/Sky/SkyGapFloorPieceBP.SkyGapFloorPieceBP_C" 4)
      (`self.QueuePieceWithVariation` "/Game/Blueprints/Objects/FloorPieces/Sky/SkyFloorPieceBP1.SkyFloorPieceBP1_C" 3)
      (`self.QueuePiece` "/Game/Blueprints/Objects/FloorPieces/Sky/SkyLeftTurnFloorPieceBP.SkyLeftTurnFloorPieceBP_C")
      (`self.QueuePieceWithVariation` "/Game/Blueprints/Objects/FloorPieces/Sky/SkyDropFloorPieceBP.SkyDropFloorPieceBP_C" 2)
      (`self.QueuePieceWithVariation` "/Game/Blueprints/Objects/FloorPieces/Sky/SkyFloorPieceBP1.SkyFloorPieceBP1_C" 1)
      (`self.QueuePieceWithVariation` "/Game/Blueprints/Objects/FloorPieces/Sky/SkyLevelEndFloorPieceBP.SkyLevelEndFloorPieceBP_C"))
    (:`12`)
    (:`13`
      ;[1 1 1] Black
      (`self.SetLevelOptions` true 1500.0 100.0 false (0.0 0.0 4684.0) (`KismetMathLibrary.MakeTransform` (100.0 0.0 75.0) (struct :`Pitch` -20.0)) false)
      (set `self.LevelFogOpacity` 0.0)
      (`self.QueuePiece` "/Game/Blueprints/Objects/FloorPieces/Platform/PlatformDownRampFloorPieceBP.PlatformDownRampFloorPieceBP_C")
      (`self.QueuePiece` "/Game/Blueprints/Objects/FloorPieces/Platform/PlatformLevelEndFloorPieceBP.PlatformLevelEndFloorPieceBP_C"))
    (:`14`
      (`self.QueuePiece` "/Game/Blueprints/Objects/FloorPieces/Special/DroppingBlocksFloorPieceBP.DroppingBlocksFloorPieceBP_C")
      (`self.QueuePiece` "/Game/Blueprints/Objects/FloorPieces/Special/LevelEndFloorPieceBP.LevelEndFloorPieceBP_C")
      (`self.SetLevelOptions` true 950.0 5.0 false (0.0 0.0 8860.0) (struct) false)
      (set `self.LevelFogOpacity` 0.0))
    (:`15`
      (`self.QueuePiece` "/Game/Blueprints/Objects/FloorPieces/Special/TunnelFloorPiece.TunnelFloorPiece_C")
      (`self.QueuePiece` "/Game/Blueprints/Objects/FloorPieces/Special/TunnelLevelEndFloorPiece.TunnelLevelEndFloorPiece_C")
      (`self.SetLevelOptions` true 2000.0 0.0 false (0.0 0.0 0.0) (struct) false)
      (set `self.LevelFogOpacity` 0.0))))

(fn `RegisterClassesBP`
  (bind _returnvalue (enumliteral `EPieceFamily` "EPF_PLATFORM"))
  (bind _returnvalue_2 (enumliteral `EPieceFamily` "EPF_CUBE"))
  (bind _returnvalue_3 (enumliteral `EPieceFamily` "EPF_WALL"))
  (bind _returnvalue_4 (enumliteral `EPieceFamily` "EPF_SKY"))
  (`|ExecutionSequence`
    (:`then_0`
      (`self.RegisterFloorPieceBPClass` "/Game/Blueprints/Objects/FloorPieces/Cube/SBendFloorPieceBP.SBendFloorPieceBP_C" 1 0.5 _returnvalue_2)
      (`self.RegisterFloorPieceBPClass` "/Game/Blueprints/Objects/FloorPieces/Cube/LeftTurnFloorPieceBP.LeftTurnFloorPieceBP_C" 1 0.5 _returnvalue_2)
      (`self.RegisterFloorPieceBPClass` "/Game/Blueprints/Objects/FloorPieces/Cube/RightTurnFloorPieceBP.RightTurnFloorPieceBP_C" 1 0.5 _returnvalue_2)
      (`self.RegisterFloorPieceBPClass` "/Game/Blueprints/Objects/FloorPieces/Cube/DoubleSBendFloorPieceBP.DoubleSBendFloorPieceBP_C" 2 0.3 _returnvalue_2)
      (`self.RegisterFloorPieceBPClass` "/Game/Blueprints/Objects/FloorPieces/Cube/SBendTightFloorPieceBP.SBendTightFloorPieceBP_C" 2 0.4 _returnvalue_2)
      (`self.RegisterFloorPieceBPClass` "/Game/Blueprints/Objects/FloorPieces/Cube/StraightFloorPieceBP.StraightFloorPieceBP_C" 1 0.5 _returnvalue_2)
      (`self.RegisterFloorPieceBPClass` "/Game/Blueprints/Objects/FloorPieces/Cube/LeftTurnFloorPieceBP2.LeftTurnFloorPieceBP2_C" 2 0.5 _returnvalue_2)
      (`self.RegisterFloorPieceBPClass` "/Game/Blueprints/Objects/FloorPieces/Cube/StraightSplitFloorPieceBP.StraightSplitFloorPieceBP_C" 2 0.1 _returnvalue_2 2)
      (`self.RegisterFloorPieceBPClass` "/Game/Blueprints/Objects/FloorPieces/Cube/UpRampFloorPieceBP.UpRampFloorPieceBP_C" 2 0.1 _returnvalue_2)
      (`self.RegisterFloorPieceBPClass` "/Game/Blueprints/Objects/FloorPieces/Cube/DownRampFloorPieceBP.DownRampFloorPieceBP_C" 2 0.1 _returnvalue_2))
    (:`then_1`
      (`self.RegisterFloorPieceBPClass` "/Game/Blueprints/Objects/FloorPieces/Indoor/IndoorFloorPieceBP.IndoorFloorPieceBP_C" 2 0.5 _returnvalue_3)
      (`self.RegisterFloorPieceBPClass` "/Game/Blueprints/Objects/FloorPieces/Indoor/ArchesFloorPieceBP.ArchesFloorPieceBP_C" 2 0.5 _returnvalue_3)
      (`self.RegisterFloorPieceBPClass` "/Game/Blueprints/Objects/FloorPieces/Indoor/TunnelsFloorPieceBP.TunnelsFloorPieceBP_C" 2 0.5 _returnvalue_3)
      (`self.RegisterFloorPieceBPClass` "/Game/Blueprints/Objects/FloorPieces/Indoor/TunnelsFloorPieceBP2.TunnelsFloorPieceBP2_C" 2 1.0 _returnvalue_3))
    (:`then_2`
      (`self.RegisterFloorPieceBPClass` "/Game/Blueprints/Objects/FloorPieces/Sky/SkyFloorPieceBP1.SkyFloorPieceBP1_C" 3 1.0 _returnvalue_4)
      (`self.RegisterFloorPieceBPClass` "/Game/Blueprints/Objects/FloorPieces/Sky/SkyCutoutFloorPieceBP2.SkyCutoutFloorPieceBP2_C" 3 0.5 _returnvalue_4)
      (`self.RegisterFloorPieceBPClass` "/Game/Blueprints/Objects/FloorPieces/Sky/SkyDropFloorPieceBP.SkyDropFloorPieceBP_C" 3 0.5 _returnvalue_4 1 "ERT_ADVANCED")
      (`self.RegisterFloorPieceBPClass` "/Game/Blueprints/Objects/FloorPieces/Sky/SkyGapFloorPieceBP.SkyGapFloorPieceBP_C" 3 0.5 _returnvalue_4))
    (:`then_3`
      (`self.RegisterFloorPieceBPClass` "/Game/Blueprints/Objects/FloorPieces/Platform/StraightPlatformFloorPieceBP.StraightPlatformFloorPieceBP_C" 4 1.0 _returnvalue)
      (`self.RegisterFloorPieceBPClass` "/Game/Blueprints/Objects/FloorPieces/Platform/DiagonalPlatformFloorPieceBP.DiagonalPlatformFloorPieceBP_C" 4 0.5 _returnvalue)
      (`self.RegisterFloorPieceBPClass` "/Game/Blueprints/Objects/FloorPieces/Platform/DiagonalPlatform2FloorPieceBP.DiagonalPlatform2FloorPieceBP_C" 4 0.5 _returnvalue)
      (`self.RegisterFloorPieceBPClass` "/Game/Blueprints/Objects/FloorPieces/Platform/JumpPlatformFloorPieceBP1.JumpPlatformFloorPieceBP1_C" 4 0.4 _returnvalue 1 "ERT_ADVANCED")
      (`self.RegisterFloorPieceBPClass` "/Game/Blueprints/Objects/FloorPieces/Platform/PlatformLeftTurnFloorPieceBP.PlatformLeftTurnFloorPieceBP_C" 4 0.4 _returnvalue))))

(fn `RegisterFamiliesBP`
  (`self.RegisterFamily` "/Game/Blueprints/Objects/FloorPieces/Special/RandomisedTransitionFloorPieceBP.RandomisedTransitionFloorPieceBP_C" "/Game/Blueprints/Objects/FloorPieces/Special/RandomisedTransitionFloorPieceBP.RandomisedTransitionFloorPieceBP_C" "EPF_RANDOMISED")
  (`self.RegisterFamily` "/Game/Blueprints/Objects/FloorPieces/Cube/CubeTransitionFloorPieceBP.CubeTransitionFloorPieceBP_C" "/Game/Blueprints/Objects/FloorPieces/Cube/CubeEndTransitionFloorPieceBP.CubeEndTransitionFloorPieceBP_C" "EPF_CUBE")
  (`self.RegisterFamilyWithLength` "/Game/Blueprints/Objects/FloorPieces/Indoor/WallTransitionFloorPieceBP.WallTransitionFloorPieceBP_C" "/Game/Blueprints/Objects/FloorPieces/Indoor/WallEndTransitionFloorPieceBP.WallEndTransitionFloorPieceBP_C" "EPF_WALL" 3 5)
  (`self.RegisterFamilyWithLength` "/Game/Blueprints/Objects/FloorPieces/Platform/PlatformStartTransitionFloorPieceBP.PlatformStartTransitionFloorPieceBP_C" "/Game/Blueprints/Objects/FloorPieces/Platform/PlatformEndTransitionFloorPieceBP.PlatformEndTransitionFloorPieceBP_C" "EPF_PLATFORM" 4 10)
  (`self.RegisterFamilyWithLength` "/Game/Blueprints/Objects/FloorPieces/Sky/SkyTransitionFloorPieceBP.SkyTransitionFloorPieceBP_C" "/Game/Blueprints/Objects/FloorPieces/Sky/SkyEndTransitionFloorPieceBP.SkyEndTransitionFloorPieceBP_C" "EPF_SKY" 3 7))

(fn `UserConstructionScript`)