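; CubeAdvancedPawnBP is a pawn Blueprint that handles tilt calibration and game menu input.
; It calls CalibrateTilt on BeginPlay.
; The OpenGameMenu action toggles the game menu, while the Android Back key explicitly shows it, both through the MainHUDWidget of CubeGameplayHUDBP on player controller 0.
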(event `self.ReceiveBeginPlay`
  (`KismetInputLibrary.CalibrateTilt`))

(event `InputAction|OpenGameMenu` :paused true
  (params (Key :type "Key Structure"))
  (:`Pressed`
    (bind _ascube_gameplay_hudbp (cast `/Game/Blueprints/UI/CubeGameplayHUDBP` (`PlayerController.GetHUD` (`GameplayStatics.GetPlayerController` 0))))
    (`/Game/Blueprints/UI/CubeGameplayHUDWidgetBP.ToggleGameMenu` (`/Game/Blueprints/UI/CubeGameplayHUDBP.MainHUDWidget` _ascube_gameplay_hudbp))))

(event `Key|Android_Back`
  (params (Key :type "Key Structure"))
  (:`Pressed`
    (bind _ascube_gameplay_hudbp (cast `/Game/Blueprints/UI/CubeGameplayHUDBP` (`PlayerController.GetHUD` (`GameplayStatics.GetPlayerController` 0))))
    (`/Game/Blueprints/UI/CubeGameplayHUDWidgetBP.ShowGameMenu` (`/Game/Blueprints/UI/CubeGameplayHUDBP.MainHUDWidget` _ascube_gameplay_hudbp) true)))

(fn `UserConstructionScript`)