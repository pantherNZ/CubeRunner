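; Game instance for the cube game that handles platform login, online highscores, achievements and default option saving.
; Login triggers leaderboard queries for Classic and Advanced modes, keeping the higher of local and online scores, and caches achievements.
; Games played is recovered from achievement progress, then stats are saved locally and increased progress is written online.
; It also notifies the menu HUD when loading finishes and opens the game menu on backgrounding.
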(event `LoadingFinishedEvent`
  (`KismetSystemLibrary.Delay` 0.1)
  (bind _asmenu_hudbp (cast `/Game/Blueprints/Menu/MenuHUDBP` (`PlayerController.GetHUD` (`GameplayStatics.GetPlayerController` 0))))
  (`/Game/Blueprints/Menu/MenuHUDBP.LoadingFinished` _asmenu_hudbp))

(event `self.OnEnteringBackground`
  (bind _ascube_gameplay_hudbp (cast `/Game/Blueprints/UI/CubeGameplayHUDBP` (`PlayerController.GetHUD` (`GameplayStatics.GetPlayerController` 0))))
  (`/Game/Blueprints/UI/CubeGameplayHUDWidgetBP.ShowGameMenu` (`/Game/Blueprints/UI/CubeGameplayHUDBP.MainHUDWidget` _ascube_gameplay_hudbp) true)
  (if true
    _
    (elif true
      _)))

(event `self.OnLoginChanged`
  (params (bLoggingIn :type Boolean) (UserID :type Integer) (UserIndex :type Integer))
  (bind _returnvalue (`GameplayStatics.GetPlayerController` 0))
  (bind _classichighscore (`self.ClassicHighscore`))
  (bind _advancedhighscore (`self.AdvancedHighscore`))
  (if bLoggingIn
    (`CubeSingletonDataLibrary.CustomLog` "Successfully logged in!" :!label _label)
    (else
      (`CubeSingletonDataLibrary.CustomLog` "Failed to log in!" "Warn" :!label _label_2)))
  (`|ExecutionSequence`
    (:`then_0`
      (bind _returnvalue_2 (`CubeSingletonDataLibrary.GetOnlineAccountID` _returnvalue :!label _label_3))
      (`self.RegisterOnlineID` _returnvalue_2)
      (`self.SaveDefaultGameOptions`)
      (`self.InitialiseAchievements`))
    (:`then_1`
      (bind _leaderboardvalue (`|LeaderboardQuery` _returnvalue "ClassicMode")
        (:`then`
          (`KismetSystemLibrary.Delay` 9.5)
          (if (not (`KismetSystemLibrary.IsLoggedIn` (`GameplayStatics.GetPlayerController` 0)))
            (`CubeSingletonDataLibrary.CustomLog` "Classic Leaderboard Timed Out " "Warn")))
        (:`OnSuccess`
          (if (> _leaderboardvalue _classichighscore)
            (set `self.ClassicHighscore` _leaderboardvalue)
            (else
              (`LeaderboardBlueprintLibrary.WriteLeaderboardInteger` _returnvalue "ClassicMode" _classichighscore :!label _label_4)))
          (bind _leaderboardvalue_2 (`|LeaderboardQuery` _returnvalue "AdvancedMode")
            (:`OnSuccess`
              (if (> _leaderboardvalue_2 _advancedhighscore)
                (set `self.AdvancedHighscore` _leaderboardvalue_2)
                (else
                  (`LeaderboardBlueprintLibrary.WriteLeaderboardInteger` _returnvalue "AdvancedMode" _advancedhighscore :!label _label_5))))
            (:`OnFailure`
              (goto _label_5)))
          (`self.HighscoresLoaded`))
        (:`OnFailure`
          (goto _label_4))))
    (:`then_2`
      (`self.InitialiseAchievements`)
      (`self.LoadingFinishedEvent`))))

(event `LoginPlatform`
  (bind _returnvalue (`GameplayStatics.GetPlayerController` 0))
  (if (`KismetSystemLibrary.IsLoggedIn` _returnvalue)
    (`self.LoadingFinishedEvent`)
    (goto _label_3)
    (else
      (`ShowLoginUICallbackProxy.ShowExternalLoginUI` _returnvalue
        (:`OnSuccess`
          (goto _label))
        (:`OnFailure`
          (goto _label_2))))))

(event `SaveDefaultGameOptions`
  (`|ExecutionSequence`
    (:`then_0`
      (bind (_loadedvalue _returnvalue) (`self.LoadCustomValue` "PlayerTiltSensitivity"))
      (if (not _returnvalue)
        (`self.SaveCustomValue` "PlayerTiltSensitivity" (/ (+ (`self.PlayerTiltSensitivityMin`) (`self.PlayerTiltSensitivityMax`)) 2.0))))
    (:`then_1`
      (bind (_loadedvalue_2 _returnvalue_2) (`self.LoadCustomBool` "MobileRotationInput"))
      (if (not _returnvalue_2)
        (`self.SaveCustomBool` "MobileRotationInput" (`self.DefaultMobileRotationInput`))))
    (:`then_2`
      (bind (_loadedvalue_3 _returnvalue_3) (`self.LoadCustomBool` "MobileRotationInput"))
      (if (not _returnvalue_3)
        (`self.SaveCustomBool` "ShowGameMenu" true)))
    (:`then_3`
      (if (or (not _returnvalue) (not _returnvalue_2) (not _returnvalue_3))
        (`self.SaveGame`)))))

(event `InitialiseAchievements`
  (bind _returnvalue (`GameplayStatics.GetPlayerController` 0))
  (`AchievementQueryCallbackProxy.CacheAchievements` _returnvalue
    (:`OnSuccess`
      (set `self.AchievementsCached` true)
      (`self.AchievementsLoaded`))
    (:`OnFailure`
      (set `self.AchievementsCached` false)))
  (for (_array_element _array_index) (`self.AchievementData`)
    (bind (_name _progress _cachedprogress) (break `Achievement` _array_element))
    (bind (_bfoundid _progress_2) (`AchievementBlueprintLibrary.GetCachedAchievementProgress` _returnvalue (`KismetStringLibrary.Conv_StringToName` _name)))
    (if _bfoundid
      (`|VariableSetRef` _progress _progress_2)
      (`|VariableSetRef` _cachedprogress (`self.ChooseLocalOrServerAchievementValue` _array_index _progress_2))
      (else
        (`CubeSingletonDataLibrary.CustomLog` (`KismetStringLibrary.Concat_StrStr` "Invalid achievement ID found: " _name) "Error"))))
  (`self.InitialiseTrackingStats`))

(event `InitialiseTrackingStats`
  (bind _stat (`self.GetStatFromAchievements` 1 1))
  (set `self.GamesPlayed` (`KismetMathLibrary.Max` (`KismetMathLibrary.FTrunc` _stat) (`self.GamesPlayed`)))
  (`self.UpdateAchievements`)
  (`LeaderboardBlueprintLibrary.WriteLeaderboardInteger` (`GameplayStatics.GetPlayerController` 0) (`KismetStringLibrary.Conv_StringToName` (`self.ClassicHighscoreSave`)) (`self.ClassicHighscore`))
  (`LeaderboardBlueprintLibrary.WriteLeaderboardInteger` (`GameplayStatics.GetPlayerController` 0) (`KismetStringLibrary.Conv_StringToName` (`self.AdvancedHighscoreSave`)) (`self.AdvancedHighscore`)))

(event `UpdateAchievements`
  (`self.SaveCustomValue` (`self.ClassicHighscoreSave`) (`KismetMathLibrary.Conv_IntToDouble` (`self.ClassicHighscore`)))
  (`self.SaveCustomValue` (`self.AdvancedHighscoreSave`) (`KismetMathLibrary.Conv_IntToDouble` (`self.AdvancedHighscore`)))
  (`self.SaveCustomValue` (`self.GamesPlayedSave`) (`KismetMathLibrary.Conv_IntToDouble` (`self.GamesPlayed`)))
  (`self.SaveCustomValue` (`self.LevelsCompleteSave`) (`KismetMathLibrary.Conv_IntToDouble` (`self.LevelsComplete`)))
  (`self.SaveGame`)
  (if (`KismetSystemLibrary.IsLoggedIn` (`GameplayStatics.GetPlayerController` 0))
    (`self.CheckAchievements` 0 0 (`KismetMathLibrary.Conv_IntToDouble` (`KismetMathLibrary.Max` (`self.ClassicHighscore`) (`self.AdvancedHighscore`))))
    (`self.CheckAchievements` 1 1 (`KismetMathLibrary.Conv_IntToDouble` (`self.GamesPlayed`)) true)))

(event `WriteAchievement`
  (params (Progress :type "Float (double-precision)") (Index :type Integer) (AchievementName :type String) (UpdateProgress :type Boolean))
  (bind (_output_name _output_progress _output_cachedprogress) (break `Achievement` (`|GetArrayItem` (`self.AchievementData`) Index)))
  (if (or (>= Progress 100.0) UpdateProgress)
    (bind (_writtenachievementname _writtenprogress) (`AchievementWriteCallbackProxy.WriteAchievementProgress` (`GameplayStatics.GetPlayerController` 0) (`KismetStringLibrary.Conv_StringToName` AchievementName) Progress)
      (:`OnSuccess`
        _)
      (:`OnFailure`
        _)))
  (`|VariableSetRef` _output_progress _writtenprogress)
  (`|VariableSetRef` _output_cachedprogress _writtenprogress))

(event `UpdateTrackingStats`)

(fn `CheckAchievements`
  (params (StartIndex :type Integer) (EndIndex :type Integer) (StatToCheckValue :type "Float (double-precision)") (UpdateProgress :type Boolean))
  (for _index (range StartIndex (+ EndIndex 1))
    (bind (_output_name _output_progress _output_cachedprogress _output_goal) (break `Achievement` (`|GetArrayItem` (`self.AchievementData`) _index)))
    (`|VariableSetRef` _output_progress (`KismetMathLibrary.FMax` (`KismetMathLibrary.FClamp` (* (/ StatToCheckValue _output_goal) 100.0) 0.0 100.0) _output_progress))
    (if (> _output_progress _output_cachedprogress)
      (`self.WriteAchievement` _output_progress _index _output_name UpdateProgress)))
  (return))

(fn `GetStatFromAchievements`
  (params (First :type Integer) (Last :type Integer))
  (returns (Stat :type "Float (double-precision)"))
  (locals (TempStat :type "Float (double-precision)"))
  (for _index (range First (+ Last 1))
    (bind (_output_name _output_progress _output_cachedprogress _output_goal) (break `Achievement` (`|GetArrayItem` (`self.AchievementData`) _index)))
    (bind (_bfoundid _progress) (`AchievementBlueprintLibrary.GetCachedAchievementProgress` (`GameplayStatics.GetPlayerController` 0) (`KismetStringLibrary.Conv_StringToName` _output_name)))
    (set `local.TempStat` (* _output_goal (/ _progress 100.0)))
    (if (< _progress 100.0)
      (break)))
  (return (`local.TempStat`)))