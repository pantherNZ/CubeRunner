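; CubePawnBP is the player's cube pawn Blueprint, mainly linking input to the in-game menu and calibrating tilt on BeginPlay.
; The OpenGameMenu action toggles the menu and Android Back shows it, both through CubeGameplayHUDBP's MainHUDWidget.
; A lost-focus handler also shows the menu, but its CubeGameInstance binding is disconnected, as is a node setting StrafeVelocity to StrafeMaxSpeed.
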(event `self.ReceiveTick`
  (params (DeltaSeconds :type "Float (single-precision)")))

(event `InputAction|OpenGameMenu` :paused true
  (params (Key :type "Key Structure"))
  (:`Pressed`
    (bind _ascube_gameplay_hudbp (cast `/Game/Blueprints/UI/CubeGameplayHUDBP` (`PlayerController.GetHUD` (`GameplayStatics.GetPlayerController` 0))))
    (`/Game/Blueprints/UI/CubeGameplayHUDWidgetBP.ToggleGameMenu` (`/Game/Blueprints/UI/CubeGameplayHUDBP.MainHUDWidget` _ascube_gameplay_hudbp))))

(event `OnLostFocus_Event`
  (bind _ascube_gameplay_hudbp (cast `/Game/Blueprints/UI/CubeGameplayHUDBP` (`PlayerController.GetHUD` (`GameplayStatics.GetPlayerController` 0))))
  (`/Game/Blueprints/UI/CubeGameplayHUDWidgetBP.ShowGameMenu` (`/Game/Blueprints/UI/CubeGameplayHUDBP.MainHUDWidget` _ascube_gameplay_hudbp) true))

(event `self.ReceiveBeginPlay`
  (`KismetInputLibrary.CalibrateTilt`))

(event `Key|Android_Back`
  (params (Key :type "Key Structure"))
  (:`Pressed`
    (bind _ascube_gameplay_hudbp (cast `/Game/Blueprints/UI/CubeGameplayHUDBP` (`PlayerController.GetHUD` (`GameplayStatics.GetPlayerController` 0))))
    (`/Game/Blueprints/UI/CubeGameplayHUDWidgetBP.ShowGameMenu` (`/Game/Blueprints/UI/CubeGameplayHUDBP.MainHUDWidget` _ascube_gameplay_hudbp) true)))

(fn `UserConstructionScript`)