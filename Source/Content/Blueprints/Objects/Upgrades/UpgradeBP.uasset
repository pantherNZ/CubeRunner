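; UpgradeBP is an upgrade object that animates itself every tick and defers its BeginPlay to the parent class.
; Its Top component spins in roll and yaw, with cosine and sine waves of game time making both speeds pulse around their base rates.
; The Sphere component's radius breathes on a slower sine wave, updating overlaps as it grows and shrinks.
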(event `self.ReceiveBeginPlay`
  (`parent.ReceiveBeginPlay`))

(event `self.ReceiveTick`
  (params (DeltaSeconds :type "Float (single-precision)"))
  (bind _returnvalue (`KismetSystemLibrary.GetGameTimeInSeconds`))
  (`SceneComponent.K2_AddRelativeRotation` (`self.Top`) (`KismetMathLibrary.MakeRotator` (* DeltaSeconds (+ (`self.RotateSpeedRoll`) (* (`self.RotateSpeedRoll`) 0.3 (`KismetMathLibrary.Cos` (* _returnvalue 5.0))))) 0.0 (* DeltaSeconds (+ (`self.RotateSpeed`) (* (`KismetMathLibrary.Sin` (* _returnvalue 5.0)) 0.3 (`self.RotateSpeed`))))) false false)
  (`SphereComponent.SetSphereRadius` (`self.Sphere`) (+ (* (`KismetMathLibrary.Sin` (`KismetSystemLibrary.GetGameTimeInSeconds`)) 125.0) 525.0) true))

(fn `UserConstructionScript`)