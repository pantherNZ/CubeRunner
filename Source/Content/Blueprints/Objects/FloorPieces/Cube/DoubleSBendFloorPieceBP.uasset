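; Floor piece Blueprint that builds a double S-bend layout of obstacles at construction time.
; Four masked, evenly spaced obstacle rows follow marker-defined control points on left and right, forming outer and inner edges that share middle start and end markers.
; Short unmasked rows line the intro and outro edges.
; The floor mesh gets a dynamic material fed its width-to-height scale ratio and a texture coordinate value.
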(fn `UserConstructionScript`
  (bind _array (`|MakeArray` 14 3 12 3))
  (bind _array_2 (`|MakeArray` 11 4 17 3))
  (bind (_returnvalue_x _returnvalue_y) (`KismetMathLibrary.BreakVector` (`SceneComponent.K2_GetComponentScale` (`self.FloorMesh`))))
  (`|ExecutionSequence`
    (:`then_0`
      (`self.SpawnObstaclesWithMask` (`|MakeArray` (`SceneComponent.K2_GetComponentLocation` (`self.RightStart_`)) (`SceneComponent.K2_GetComponentLocation` (`self.RightMiddle11Marker`)) (`SceneComponent.K2_GetComponentLocation` (`self.RightMiddle22Marker`)) (`SceneComponent.K2_GetComponentLocation` (`self.RightMiddle33Marker`)) (`SceneComponent.K2_GetComponentLocation` (`self.RightEndMarker`))) 50 "ESOAT_FOLLOW_ROTATION" _array 0 true)
      (`self.SpawnObstaclesWithMask` (`|MakeArray` (`SceneComponent.K2_GetComponentLocation` (`self.MiddleStart_`)) (`SceneComponent.K2_GetComponentLocation` (`self.RightMiddle1Marker`)) (`SceneComponent.K2_GetComponentLocation` (`self.RightMiddle2Marker`)) (`SceneComponent.K2_GetComponentLocation` (`self.RightMiddle3Marker`)) (`SceneComponent.K2_GetComponentLocation` (`self.EndMiddleMarker`))) 50 "ESOAT_FOLLOW_ROTATION" _array_2 0 true))
    (:`then_1`
      (bind _returnvalue (`PrimitiveComponent.CreateDynamicMaterialInstance` (`self.FloorMesh`) 0 "/Game/Materials/TestFloor.TestFloor"))
      (`MaterialInstanceDynamic.SetScalarParameterValue` _returnvalue "WidthToHeightRatio" (/ _returnvalue_x _returnvalue_y))
      (`MaterialInstanceDynamic.SetScalarParameterValue` _returnvalue "TexCoord" 20.0))
    (:`then_2`
      (`self.SpawnObstaclesWithMask` (`|MakeArray` (`SceneComponent.K2_GetComponentLocation` (`self.LeftStart_`)) (`SceneComponent.K2_GetComponentLocation` (`self.LeftMiddle1Marker`)) (`SceneComponent.K2_GetComponentLocation` (`self.LeftMiddle2Marker`)) (`SceneComponent.K2_GetComponentLocation` (`self.LeftMiddle3Marker`)) (`SceneComponent.K2_GetComponentLocation` (`self.LeftEndMarker`))) 50 "ESOAT_FOLLOW_ROTATION" _array 0 true)
      (`self.SpawnObstaclesWithMask` (`|MakeArray` (`SceneComponent.K2_GetComponentLocation` (`self.MiddleStart_`)) (`SceneComponent.K2_GetComponentLocation` (`self.LeftMiddle11Marker`)) (`SceneComponent.K2_GetComponentLocation` (`self.LeftMiddle22Marker`)) (`SceneComponent.K2_GetComponentLocation` (`self.LeftMiddle33Marker`)) (`SceneComponent.K2_GetComponentLocation` (`self.EndMiddleMarker`))) 50 "ESOAT_FOLLOW_ROTATION" _array_2 0 true))
    (:`then_3`
      (`self.SpawnObstacles` (`|MakeArray` (`SceneComponent.K2_GetComponentLocation` (`self.LeftStartStart_`)) (`SceneComponent.K2_GetComponentLocation` (`self.IntroLeftMidMarker`)) (`SceneComponent.K2_GetComponentLocation` (`self.LeftStart_`))) 3 "ESOAT_FOLLOW_ROTATION")
      (`self.SpawnObstacles` (`|MakeArray` (`SceneComponent.K2_GetComponentLocation` (`self.RightStartStart_`)) (`SceneComponent.K2_GetComponentLocation` (`self.IntroRightMidMarker`)) (`SceneComponent.K2_GetComponentLocation` (`self.RightStart_`))) 3 "ESOAT_FOLLOW_ROTATION")
      (`self.SpawnObstacles` (`|MakeArray` (`SceneComponent.K2_GetComponentLocation` (`self.LeftEndMarker`)) (`SceneComponent.K2_GetComponentLocation` (`self.OutroMidLeftMarker`)) (`SceneComponent.K2_GetComponentLocation` (`self.LeftEndEnd_`))) 3 "ESOAT_FOLLOW_ROTATION")
      (`self.SpawnObstacles` (`|MakeArray` (`SceneComponent.K2_GetComponentLocation` (`self.RightEndMarker`)) (`SceneComponent.K2_GetComponentLocation` (`self.OutroMidRightMarker`)) (`SceneComponent.K2_GetComponentLocation` (`self.RightEndEnd_`))) 3 "ESOAT_FOLLOW_ROTATION"))))