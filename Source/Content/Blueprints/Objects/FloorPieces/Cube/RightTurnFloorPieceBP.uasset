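; Right-turn floor piece Blueprint that builds a curved track section with obstacles along its left and right edges.
; The construction script gives the floor mesh a dynamic material corrected for its scale ratio.
; It then derives control points for each side of the turn and spawns rotation-following obstacles along them, with more, evenly spaced ones on the left.
; On begin play, it passes two markers to a variation obstacle as dynamic waypoints, if present.
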(event `self.OnFloorPieceBeginPlay`
  (bind _variationobstacle1 (`self.VariationObstacle1`))
  (`/Engine/EditorBlueprintResources/StandardMacros.IsValid` _variationobstacle1
    (:`Is Valid`
      (`BaseObstacleComponent.AddDynamicWaypoints` _variationobstacle1 (`self.Marker1`) (`self.Marker2`)))))

(fn `UserConstructionScript`
  (bind (_returnvalue_x _returnvalue_y) (`KismetMathLibrary.BreakVector` (`SceneComponent.K2_GetComponentScale` (`self.FloorMesh`))))
  (`|ExecutionSequence`
    (:`then_0`
      (bind _returnvalue (`PrimitiveComponent.CreateDynamicMaterialInstance` (`self.FloorMesh`) 0 "/Game/Materials/TestFloor.TestFloor"))
      (`MaterialInstanceDynamic.SetScalarParameterValue` _returnvalue "WidthToHeightRatio" (/ _returnvalue_x _returnvalue_y))
      (`MaterialInstanceDynamic.SetScalarParameterValue` _returnvalue "TexCoord" 20.0))
    (:`then_1`
      (bind _returnvalue_2 (`self.FindTurnControlPoints` (`self.TurnLeftStart`) (`self.TurnLeftEnd`)))
      (`self.SpawnObstacles` _returnvalue_2 22 "ESOAT_FOLLOW_ROTATION" 0 true))
    (:`then_2`
      (bind _returnvalue_3 (`self.FindTurnControlPoints` (`self.TurnRightStart`) (`self.TurnRightEnd`)))
      (`self.SpawnObstacles` _returnvalue_3 15 "ESOAT_FOLLOW_ROTATION"))))