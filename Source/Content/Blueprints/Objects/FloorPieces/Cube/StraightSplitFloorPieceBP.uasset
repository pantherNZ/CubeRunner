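; Straight floor piece that splits into two branches, registering Connection2 and its Box collider as a multi-connection at begin play.
; The construction script sets up an aspect-corrected floor material and, if Wall is valid, randomly moves it to one of two mirrored, hard-coded world-space transforms.
; It then spawns rotation-following obstacles along four control-point paths: evenly spaced on both outer edges, plus two forking from the middle start.
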(event `self.OnFloorPieceBeginPlay`
  (`self.AddMultiConnection` (`self.Connection2`) (`self.Box`)))

(fn `UserConstructionScript`
  (bind _wall (`self.Wall`))
  (bind (_returnvalue_x _returnvalue_y) (`KismetMathLibrary.BreakVector` (`SceneComponent.K2_GetComponentScale` (`self.FloorMesh`))))
  (`|ExecutionSequence`
    (:`then_0`
      (bind _returnvalue (`PrimitiveComponent.CreateDynamicMaterialInstance` (`self.FloorMesh`) 0 "/Game/Materials/TestFloor.TestFloor"))
      (`MaterialInstanceDynamic.SetScalarParameterValue` _returnvalue "WidthToHeightRatio" (/ _returnvalue_x _returnvalue_y))
      (`MaterialInstanceDynamic.SetScalarParameterValue` _returnvalue "TexCoord" 20.0)
      (`/Engine/EditorBlueprintResources/StandardMacros.IsValid` _wall
        (:`Is Valid`
          (if (`KismetMathLibrary.RandomBool`)
            (`SceneComponent.K2_SetWorldLocationAndRotation` _wall (2900.0 1800.0 0.0) (struct :`Yaw` 40.0) false false)
            (else
              (`SceneComponent.K2_SetWorldLocationAndRotation` _wall (2900.0 -1850.0 0.0) (struct :`Yaw` -40.0) false false))))))
    (:`then_1`
      (`self.SpawnObstacles` (`|MakeArray` (`SceneComponent.K2_GetComponentLocation` (`self.StartLeft`)) (`SceneComponent.K2_GetComponentLocation` (`self.LeftMiddle1`)) (`SceneComponent.K2_GetComponentLocation` (`self.LeftMiddle2`)) (`SceneComponent.K2_GetComponentLocation` (`self.EndLeft`))) 29 "ESOAT_FOLLOW_ROTATION" 0 true))
    (:`then_2`
      (`self.SpawnObstacles` (`|MakeArray` (`SceneComponent.K2_GetComponentLocation` (`self.StartRight`)) (`SceneComponent.K2_GetComponentLocation` (`self.RightMiddle1`)) (`SceneComponent.K2_GetComponentLocation` (`self.RightMiddle2`)) (`SceneComponent.K2_GetComponentLocation` (`self.EndRight`))) 29 "ESOAT_FOLLOW_ROTATION" 0 true))
    (:`then_3`
      (`self.SpawnObstacles` (`|MakeArray` (`SceneComponent.K2_GetComponentLocation` (`self.StartMiddle`)) (`SceneComponent.K2_GetComponentLocation` (`self.MiddleLeft`)) (`SceneComponent.K2_GetComponentLocation` (`self.MiddleLeftEnd`))) 19 "ESOAT_FOLLOW_ROTATION"))
    (:`then_4`
      (`self.SpawnObstacles` (`|MakeArray` (`SceneComponent.K2_GetComponentLocation` (`self.StartMiddle`)) (`SceneComponent.K2_GetComponentLocation` (`self.MiddleRight`)) (`SceneComponent.K2_GetComponentLocation` (`self.MiddleRightEnd`))) 19 "ESOAT_FOLLOW_ROTATION"))))