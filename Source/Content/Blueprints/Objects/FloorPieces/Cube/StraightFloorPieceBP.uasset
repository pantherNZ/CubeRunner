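; Straight floor piece Blueprint that builds its own obstacle layout and gives its Variation 1 obstacles dynamic waypoints.
; The construction script spawns obstacle rows between left and right edge markers, plus a variation-specific row of cube obstacles between two other markers.
; It also creates a dynamic floor material that receives the mesh's scale ratio and texture tiling.
; On floor piece begin play, four valid obstacles each receive successive marker pairs as waypoints.
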(event `self.OnFloorPieceBeginPlay`
  (bind _variation1obstacle2 (`self.Variation1Obstacle2`))
  (bind _variation1obstacle1 (`self.Variation1Obstacle1`))
  (bind _variation1obstacle3 (`self.Variation1Obstacle3`))
  (bind _variation1obstacle4 (`self.Variation1Obstacle4`))
  (`|ExecutionSequence`
    (:`then_0`
      (`/Engine/EditorBlueprintResources/StandardMacros.IsValid` _variation1obstacle1
        (:`Is Valid`
          (`BaseObstacleComponent.AddDynamicWaypoints` _variation1obstacle1 (`self.Marker1`) (`self.Marker2`)))))
    (:`then_1`
      (`/Engine/EditorBlueprintResources/StandardMacros.IsValid` _variation1obstacle2
        (:`Is Valid`
          (`BaseObstacleComponent.AddDynamicWaypoints` _variation1obstacle2 (`self.Marker2`) (`self.Marker3`)))))
    (:`then_2`
      (`/Engine/EditorBlueprintResources/StandardMacros.IsValid` _variation1obstacle3
        (:`Is Valid`
          (`BaseObstacleComponent.AddDynamicWaypoints` _variation1obstacle3 (`self.Marker3`) (`self.Marker4`)))))
    (:`then_3`
      (`/Engine/EditorBlueprintResources/StandardMacros.IsValid` _variation1obstacle4
        (:`Is Valid`
          (`BaseObstacleComponent.AddDynamicWaypoints` _variation1obstacle4 (`self.Marker4`) (`self.Marker5`)))))))

(fn `UserConstructionScript`
  (bind (_returnvalue_x _returnvalue_y) (`KismetMathLibrary.BreakVector` (`SceneComponent.K2_GetComponentScale` (`self.FloorMesh`))))
  (`self.SpawnObstacles` (`|MakeArray` (`SceneComponent.K2_GetComponentLocation` (`self.StartLeftMarker`)) (`SceneComponent.K2_GetComponentLocation` (`self.EndLeftMarker`))) 18 "ESOAT_DEFAULT")
  (`self.SpawnObstacles` (`|MakeArray` (`SceneComponent.K2_GetComponentLocation` (`self.StartRightMarker`)) (`SceneComponent.K2_GetComponentLocation` (`self.EndRightMarker`))) 18 "ESOAT_DEFAULT")
  (bind _returnvalue (`PrimitiveComponent.CreateDynamicMaterialInstance` (`self.FloorMesh`) 0 "/Game/Materials/TestFloor.TestFloor"))
  (`MaterialInstanceDynamic.SetScalarParameterValue` _returnvalue "WidthToHeightRatio" (/ _returnvalue_x _returnvalue_y))
  (`MaterialInstanceDynamic.SetScalarParameterValue` _returnvalue "TexCoord" 20.0)
  (`self.SpawnObstacles` (`|MakeArray` (`SceneComponent.K2_GetComponentLocation` (`self.MarkerComponent`)) (`SceneComponent.K2_GetComponentLocation` (`self.MarkerComponent1`))) 5 "ESOAT_DEFAULT" 6 false "/Game/Blueprints/Objects/Obstacles/CubeObstacleComponentBP.CubeObstacleComponentBP_C"))