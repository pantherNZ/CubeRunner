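; Tight S-bend floor piece that builds its floor material and edge obstacles in the construction script, with no active event graph logic.
; A dynamic floor material instance receives the mesh's width-to-height scale ratio and a fixed texture coordinate value.
; Left and right rows of marker components supply control points to SpawnObstacles, which places evenly spaced, rotation-following obstacles along each side of the bend.
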(fn `UserConstructionScript`
  (bind (_returnvalue_x _returnvalue_y) (`KismetMathLibrary.BreakVector` (`SceneComponent.K2_GetComponentScale` (`self.FloorMesh`))))
  (`|ExecutionSequence`
    (:`then_0`
      (bind _returnvalue (`PrimitiveComponent.CreateDynamicMaterialInstance` (`self.FloorMesh`) 0 "/Game/Materials/TestFloor.TestFloor"))
      (`MaterialInstanceDynamic.SetScalarParameterValue` _returnvalue "WidthToHeightRatio" (/ _returnvalue_x _returnvalue_y))
      (`MaterialInstanceDynamic.SetScalarParameterValue` _returnvalue "TexCoord" 20.0))
    (:`then_1`
      (`self.SpawnObstacles` (`|MakeArray` (`SceneComponent.K2_GetComponentLocation` (`self.StartLeft_`)) (`SceneComponent.K2_GetComponentLocation` (`self.LeftMiddle1Marker`)) (`SceneComponent.K2_GetComponentLocation` (`self.LeftMiddle2Marker`)) (`SceneComponent.K2_GetComponentLocation` (`self.LeftMiddle3Marker`)) (`SceneComponent.K2_GetComponentLocation` (`self.LeftMiddle4Marker`)) (`SceneComponent.K2_GetComponentLocation` (`self.EndLeftMarker`))) 42 "ESOAT_FOLLOW_ROTATION" 0 true))
    (:`then_2`
      (`self.SpawnObstacles` (`|MakeArray` (`SceneComponent.K2_GetComponentLocation` (`self.StartRight_`)) (`SceneComponent.K2_GetComponentLocation` (`self.RightMiddle1Marker`)) (`SceneComponent.K2_GetComponentLocation` (`self.RightMiddle2Marker`)) (`SceneComponent.K2_GetComponentLocation` (`self.RightMiddle3Marker`)) (`SceneComponent.K2_GetComponentLocation` (`self.RightMiddle4Marker`)) (`SceneComponent.K2_GetComponentLocation` (`self.EndRightMarker`))) 42 "ESOAT_FOLLOW_ROTATION" 0 true))))