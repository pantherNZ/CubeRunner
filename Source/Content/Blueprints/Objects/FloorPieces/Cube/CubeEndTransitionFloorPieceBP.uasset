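; CubeEndTransitionFloorPieceBP is a cube-themed end transition floor piece, built entirely in its construction script.
; It gives FloorMesh a dynamic TestFloor material, feeding in the mesh's X/Y scale ratio and a fixed TexCoord.
; It then calls SpawnObstacles for the left and right sides, placing evenly spaced, rotation-following obstacles through start, middle and end marker control points.
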(fn `UserConstructionScript`
  (bind (_returnvalue_x _returnvalue_y) (`KismetMathLibrary.BreakVector` (`SceneComponent.K2_GetComponentScale` (`self.FloorMesh`))))
  (`|ExecutionSequence`
    (:`then_0`
      (bind _returnvalue (`PrimitiveComponent.CreateDynamicMaterialInstance` (`self.FloorMesh`) 0 "/Game/Materials/TestFloor.TestFloor"))
      (`MaterialInstanceDynamic.SetScalarParameterValue` _returnvalue "WidthToHeightRatio" (/ _returnvalue_x _returnvalue_y))
      (`MaterialInstanceDynamic.SetScalarParameterValue` _returnvalue "TexCoord" 20.0))
    (:`then_1`
      (`self.SpawnObstacles` (`|MakeArray` (`SceneComponent.K2_GetComponentLocation` (`self.LeftStart`)) (`SceneComponent.K2_GetComponentLocation` (`self.MiddleLeftMarker`)) (`SceneComponent.K2_GetComponentLocation` (`self.LeftEnd`))) 35 "ESOAT_FOLLOW_ROTATION" 0 true))
    (:`then_2`
      (`self.SpawnObstacles` (`|MakeArray` (`SceneComponent.K2_GetComponentLocation` (`self.RightStart`)) (`SceneComponent.K2_GetComponentLocation` (`self.MiddleRightMarker`)) (`SceneComponent.K2_GetComponentLocation` (`self.RightEnd`))) 35 "ESOAT_FOLLOW_ROTATION" 0 true))))