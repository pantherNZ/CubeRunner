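; Cube transition floor piece that builds its floor material and lines both sides with obstacles in the Construction Script.
; A dynamic material instance on the floor mesh receives the mesh's width-to-height scale ratio and a texture coordinate value.
; Marker component locations feed SpawnObstacles as control points, placing an evenly spaced, rotation-following Bezier row plus a second two-point row on each side.
; The event graph holds no active logic.
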(fn `UserConstructionScript`
  (bind _returnvalue (`SceneComponent.K2_GetComponentLocation` (`self.StartRightMarker`)))
  (bind (_returnvalue_x _returnvalue_y) (`KismetMathLibrary.BreakVector` (`SceneComponent.K2_GetComponentScale` (`self.FloorMesh`))))
  (bind _returnvalue_2 (`SceneComponent.K2_GetComponentLocation` (`self.StartLeftMarker`)))
  (`|ExecutionSequence`
    (:`then_0`
      (bind _returnvalue_3 (`PrimitiveComponent.CreateDynamicMaterialInstance` (`self.FloorMesh`) 0 "/Game/Materials/TestFloor.TestFloor"))
      (`MaterialInstanceDynamic.SetScalarParameterValue` _returnvalue_3 "WidthToHeightRatio" (/ _returnvalue_x _returnvalue_y))
      (`MaterialInstanceDynamic.SetScalarParameterValue` _returnvalue_3 "TexCoord" 20.0))
    (:`then_1`
      (`self.SpawnObstacles` (`|MakeArray` _returnvalue (`SceneComponent.K2_GetComponentLocation` (`self.MarkerComponent1`)) (`SceneComponent.K2_GetComponentLocation` (`self.MiddleRightMarker`)) (`SceneComponent.K2_GetComponentLocation` (`self.EndRightMarker`))) 42 "ESOAT_FOLLOW_ROTATION" 0 true null 300)
      (`self.SpawnObstacles` (`|MakeArray` _returnvalue (`SceneComponent.K2_GetComponentLocation` (`self.StartRightMarker2`))) 20 "ESOAT_FOLLOW_ROTATION" 0 false null 0))
    (:`then_2`
      (`self.SpawnObstacles` (`|MakeArray` _returnvalue_2 (`SceneComponent.K2_GetComponentLocation` (`self.MarkerComponent`)) (`SceneComponent.K2_GetComponentLocation` (`self.MiddleLeftMarker`)) (`SceneComponent.K2_GetComponentLocation` (`self.EndLeftMarker`))) 42 "ESOAT_FOLLOW_ROTATION" 0 true null 300)
      (`self.SpawnObstacles` (`|MakeArray` _returnvalue_2 (`SceneComponent.K2_GetComponentLocation` (`self.StartLeftMarker2`))) 20 "ESOAT_FOLLOW_ROTATION" 0 false null 0))))