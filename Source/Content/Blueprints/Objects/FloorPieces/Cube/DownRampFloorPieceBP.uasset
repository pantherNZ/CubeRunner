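; Down-ramp floor piece Blueprint that assembles its edge obstacles and floor material in the construction script.
; It spawns two evenly counted rows of attached obstacles, using the left and right start and end markers as control points.
; The floor mesh gets a dynamic TestFloor material instance, fed the mesh's world X-to-Y scale ratio and a fixed texture-coordinate value.
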(fn `UserConstructionScript`
  (bind (_returnvalue_x _returnvalue_y) (`KismetMathLibrary.BreakVector` (`SceneComponent.K2_GetComponentScale` (`self.FloorMesh`))))
  (`|ExecutionSequence`
    (:`then_0`
      (`self.SpawnObstacles` (`|MakeArray` (`SceneComponent.K2_GetComponentLocation` (`self.StartLeftMarker`)) (`SceneComponent.K2_GetComponentLocation` (`self.EndLeftMarker2`))) 35 "ESOAT_ATTACH")
      (`self.SpawnObstacles` (`|MakeArray` (`SceneComponent.K2_GetComponentLocation` (`self.StartRightMarker`)) (`SceneComponent.K2_GetComponentLocation` (`self.EndRightMarker2`))) 35 "ESOAT_ATTACH")
      (bind _returnvalue (`PrimitiveComponent.CreateDynamicMaterialInstance` (`self.FloorMesh`) 0 "/Game/Materials/TestFloor.TestFloor"))
      (`MaterialInstanceDynamic.SetScalarParameterValue` _returnvalue "WidthToHeightRatio" (/ _returnvalue_x _returnvalue_y))
      (`MaterialInstanceDynamic.SetScalarParameterValue` _returnvalue "TexCoord" 20.0))))