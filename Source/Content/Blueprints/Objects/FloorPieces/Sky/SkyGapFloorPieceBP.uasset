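; Sky floor piece with a gap, built from three meshes and set up entirely in its construction script.
; Each mesh gets a dynamic TestFloor material instance, fed its world X/Y scale ratio and a fixed TexCoord value.
; A random boolean then puts StaticMesh1 at one of two mirrored Y offsets, so its side can change whenever construction runs.
; The event graph holds no active logic.
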(fn `UserConstructionScript`
  (bind _staticmesh1 (`self.StaticMesh1`))
  (bind (_returnvalue_x _returnvalue_y) (`KismetMathLibrary.BreakVector` (`SceneComponent.K2_GetComponentScale` (`self.StaticMesh1`))))
  (bind (_returnvalue_x_2 _returnvalue_y_2) (`KismetMathLibrary.BreakVector` (`SceneComponent.K2_GetComponentScale` (`self.FloorMesh`))))
  (bind (_returnvalue_x_3 _returnvalue_y_3) (`KismetMathLibrary.BreakVector` (`SceneComponent.K2_GetComponentScale` (`self.StaticMesh`))))
  (`|ExecutionSequence`
    (:`then_0`
      (bind _returnvalue (`PrimitiveComponent.CreateDynamicMaterialInstance` (`self.FloorMesh`) 0 "/Game/Materials/TestFloor.TestFloor"))
      (`MaterialInstanceDynamic.SetScalarParameterValue` _returnvalue "WidthToHeightRatio" (/ _returnvalue_x_2 _returnvalue_y_2))
      (`MaterialInstanceDynamic.SetScalarParameterValue` _returnvalue "TexCoord" 20.0)
      (bind _returnvalue_2 (`PrimitiveComponent.CreateDynamicMaterialInstance` (`self.StaticMesh`) 0 "/Game/Materials/TestFloor.TestFloor"))
      (`MaterialInstanceDynamic.SetScalarParameterValue` _returnvalue_2 "WidthToHeightRatio" (/ _returnvalue_x_3 _returnvalue_y_3))
      (`MaterialInstanceDynamic.SetScalarParameterValue` _returnvalue_2 "TexCoord" 20.0)
      (bind _returnvalue_3 (`PrimitiveComponent.CreateDynamicMaterialInstance` (`self.StaticMesh1`) 0 "/Game/Materials/TestFloor.TestFloor"))
      (`MaterialInstanceDynamic.SetScalarParameterValue` _returnvalue_3 "WidthToHeightRatio" (/ _returnvalue_x _returnvalue_y))
      (`MaterialInstanceDynamic.SetScalarParameterValue` _returnvalue_3 "TexCoord" 20.0))
    (:`then_1`
      (if (`KismetMathLibrary.RandomBool`)
        (`SceneComponent.K2_SetRelativeLocation` _staticmesh1 (2500.0 -350.0 -5000.0) false false)
        (else
          (`SceneComponent.K2_SetRelativeLocation` _staticmesh1 (2500.0 350.0 -5000.0) false false))))))