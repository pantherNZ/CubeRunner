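; Sky-themed drop floor piece, with a ConnectionPoint that the Variation value positions at its far end.
; The construction script gives both meshes dynamic TestFloor materials, feeding each mesh's X/Y scale ratio and a fixed TexCoord into them.
; It then offsets ConnectionPoint by Variation: lowered straight, lowered to either side, or straight at zero height.
; All logic runs at construction, as the event graph is empty.
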(fn `UserConstructionScript`
  (bind _connectionpoint (`self.ConnectionPoint`))
  (bind (_returnvalue_x _returnvalue_y) (`KismetMathLibrary.BreakVector` (`SceneComponent.K2_GetComponentScale` (`self.FloorMesh`))))
  (bind (_returnvalue_x_2 _returnvalue_y_2) (`KismetMathLibrary.BreakVector` (`SceneComponent.K2_GetComponentScale` (`self.StaticMesh`))))
  (`|ExecutionSequence`
    (:`then_0`
      (bind _returnvalue (`PrimitiveComponent.CreateDynamicMaterialInstance` (`self.FloorMesh`) 0 "/Game/Materials/TestFloor.TestFloor"))
      (`MaterialInstanceDynamic.SetScalarParameterValue` _returnvalue "WidthToHeightRatio" (/ _returnvalue_x _returnvalue_y))
      (`MaterialInstanceDynamic.SetScalarParameterValue` _returnvalue "TexCoord" 20.0)
      (bind _returnvalue_2 (`PrimitiveComponent.CreateDynamicMaterialInstance` (`self.StaticMesh`) 0 "/Game/Materials/TestFloor.TestFloor"))
      (`MaterialInstanceDynamic.SetScalarParameterValue` _returnvalue_2 "WidthToHeightRatio" (/ _returnvalue_x_2 _returnvalue_y_2))
      (`MaterialInstanceDynamic.SetScalarParameterValue` _returnvalue_2 "TexCoord" 20.0))
    (:`then_1`
      (switch `int` (`self.Variation`)
        (:`0`
          (`SceneComponent.K2_SetRelativeLocation` _connectionpoint (7000.0 0.0 -480.0) false false))
        (:`1`
          (`SceneComponent.K2_SetRelativeLocation` _connectionpoint (7000.0 1000.0 -480.0) false false))
        (:`2`
          (`SceneComponent.K2_SetRelativeLocation` _connectionpoint (7000.0 -1000.0 -480.0) false false))
        (:`3`
          (`SceneComponent.K2_SetRelativeLocation` _connectionpoint (7000.0 0.0 0.0) false false))))))