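; Indoor wall-transition floor piece that fades out the level fog when the player passes through it.
; Overlap of the FogFadeStart trigger by a BasePlayerPawn gets the fog actor from CubeGameModeBP and starts the fade.
; Tick then lowers the fog's max opacity at FogFadeSpeed until it reaches FogMin.
; The construction script gives the floor mesh a dynamic material that receives its width-to-height scale ratio and texture coordinate scale.
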(event `self.FogFadeStart.OnComponentBeginOverlap`
  (params (OverlappedComponent :type "PrimitiveComponent Object Reference") (OtherActor :type "Actor Object Reference") (OtherComp :type "PrimitiveComponent Object Reference") (OtherBodyIndex :type Integer) (bFromSweep :type Boolean) (SweepResult :type "HitResult Structure (by ref)"))
  (cast `BasePlayerPawn` OtherActor)
  (bind _ascube_game_mode_bp (cast `/Game/Blueprints/Core/CubeGameModeBP` (`GameplayStatics.GetGameMode`)))
  (bind _fog (`/Game/Blueprints/Core/CubeGameModeBP.GetFogActor` _ascube_game_mode_bp))
  (set `self.FogActor` _fog)
  (set `self.FadeFog` true))

(event `self.ReceiveTick`
  (params (DeltaSeconds :type "Float (single-precision)"))
  (bind _fogmin (`self.FogMin`))
  (bind _component (`ExponentialHeightFog.Component` (`self.FogActor`)))
  (bind _returnvalue (`KismetMathLibrary.FMax` (- (`ExponentialHeightFogComponent.FogMaxOpacity` _component) (* DeltaSeconds (`self.FogFadeSpeed`))) _fogmin))
  (if (`self.FadeFog`)
    (`ExponentialHeightFogComponent.SetFogMaxOpacity` _component _returnvalue)
    (if (<= _returnvalue _fogmin)
      (set `self.FadeFog` false))))

(fn `UserConstructionScript`
  (bind (_returnvalue_x _returnvalue_y) (`KismetMathLibrary.BreakVector` (`SceneComponent.K2_GetComponentScale` (`self.FloorMesh`))))
  (bind _returnvalue (`PrimitiveComponent.CreateDynamicMaterialInstance` (`self.FloorMesh`) 0 "/Game/Materials/TestFloor.TestFloor"))
  (`MaterialInstanceDynamic.SetScalarParameterValue` _returnvalue "WidthToHeightRatio" (/ _returnvalue_x _returnvalue_y))
  (`MaterialInstanceDynamic.SetScalarParameterValue` _returnvalue "TexCoord" 20.0))