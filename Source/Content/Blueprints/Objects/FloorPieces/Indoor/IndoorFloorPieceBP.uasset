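; IndoorFloorPieceBP is an indoor floor piece actor with a floor mesh and a right wall child actor.
; Its construction script gives the mesh a dynamic TestFloor material, setting texture tiling and a width-to-height ratio from the mesh's world X/Y scale.
; On BeginPlay it casts the WallRight child actor to BaseWallPiece and clears its LeftWall flag, marking it as the right-hand wall.
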(event `self.ReceiveBeginPlay`
  (bind _asbase_wall_piece (cast `BaseWallPiece` (`ChildActorComponent.ChildActor` (`self.WallRight`))))
  (set `BaseWallPiece.LeftWall` false _asbase_wall_piece))

(fn `UserConstructionScript`
  (bind (_returnvalue_x _returnvalue_y) (`KismetMathLibrary.BreakVector` (`SceneComponent.K2_GetComponentScale` (`self.FloorMesh`))))
  (bind _returnvalue (`PrimitiveComponent.CreateDynamicMaterialInstance` (`self.FloorMesh`) 0 "/Game/Materials/TestFloor.TestFloor"))
  (`MaterialInstanceDynamic.SetScalarParameterValue` _returnvalue "WidthToHeightRatio" (/ _returnvalue_x _returnvalue_y))
  (`MaterialInstanceDynamic.SetScalarParameterValue` _returnvalue "TexCoord" 20.0))