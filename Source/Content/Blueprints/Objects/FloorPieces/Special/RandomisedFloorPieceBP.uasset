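; Randomised floor piece Blueprint that tints its cube obstacles according to its Variation value.
; On floor piece begin play, a positive Variation is mapped to a rainbow colour, applied through a dynamic material to the cube obstacles' instanced static mesh, recolouring all instances together.
; The construction script gives the floor a dynamic test material, passing the mesh's X/Y scale ratio and a fixed texture coordinate value.
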(event `self.OnFloorPieceBeginPlay`
  (bind (_value _returnvalue) (`BlueprintMapLibrary.Map_Find` (`self.InstancedObstacleData`) "/Game/Meshes/Shape_Cube_Obstacle.Shape_Cube_Obstacle"))
  (if (> (`self.Variation`) 0)
    (if _returnvalue
      (bind _returnvalue_2 (`KismetMaterialLibrary.CreateDynamicMaterialInstance` "/Game/Materials/Colour_Mat.Colour_Mat"))
      (bind _returnvalue_3 (`CubeSingletonDataLibrary.GetRainbowColour` (`self.Variation`) 20))
      (`MaterialInstanceDynamic.SetVectorParameterValue` _returnvalue_2 "Colour" (make `LinearColor` (.x _returnvalue_3) (.y _returnvalue_3) (.z _returnvalue_3) 1.0))
      (`PrimitiveComponent.SetMaterial` (`.InstancedStaticMesh` (break `InstancedObstacleDataContainer` _value)) 0 _returnvalue_2))))

(fn `UserConstructionScript`
  (bind (_returnvalue_x _returnvalue_y) (`KismetMathLibrary.BreakVector` (`SceneComponent.K2_GetComponentScale` (`self.FloorMesh`))))
  (bind _returnvalue (`PrimitiveComponent.CreateDynamicMaterialInstance` (`self.FloorMesh`) 0 "/Game/Materials/TestFloor.TestFloor"))
  (`MaterialInstanceDynamic.SetScalarParameterValue` _returnvalue "WidthToHeightRatio" (/ _returnvalue_x _returnvalue_y))
  (`MaterialInstanceDynamic.SetScalarParameterValue` _returnvalue "TexCoord" 20.0))